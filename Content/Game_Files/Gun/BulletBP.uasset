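; Gun projectile that spawns trampolines on tagged surfaces and knocks objective cubes around.
; On hit it branches by actor tag: objectives get a velocity-based impulse and refund a round, spawn surfaces get a trampoline oriented from the hit normal, and existing trampolines just play a sound.
; It registers itself with the player character, clears BulletInAir or calls ResetBall when finished, and expires after a short delay if still airborne.
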(event `Hit Tramp`
  ;[1 1 1] Hit Trampoline
  (`KismetSystemLibrary.PrintString` "Hello")
  (`GameplayStatics.PlaySoundAtLocation` "/Game/Game_Files/SFX/Trampoline/sci-fi_electric_pulse_power_down_01.sci-fi_electric_pulse_power_down_01" (`self.K2_GetActorLocation`) (struct) 0.3 (`KismetMathLibrary.RandomFloatInRange` 0.65 1.35) 0.0 "/Game/Game_Files/SFX/DistanceSFX.DistanceSFX" null null)
  (bind _asue_4asp_character (cast `/Game/Game_Files/Character/Ue4ASP_Character` (`GameplayStatics.GetPlayerCharacter` 0)))
  (set `/Game/Game_Files/Character/Ue4ASP_Character.BulletInAir?` false _asue_4asp_character)
  (`self.K2_DestroyActor`))

(event `Hit Objective`
  ;[1 1 1] Launch Object
  (bind _asobjective_cube (cast `/Game/Game_Files/Objective/ObjectiveCube` (stale `self.ReceiveHit` Other)))
  (`PrimitiveComponent.AddImpulseAtLocation` (`/Game/Game_Files/Objective/ObjectiveCube.Box` _asobjective_cube) (* (`self.GetVelocity`) 15.0) (`self.K2_GetActorLocation`) "None")
  (`GameplayStatics.PlaySoundAtLocation` "/Game/Game_Files/SFX/Weapon/MetalImpact.MetalImpact" (`self.K2_GetActorLocation`) (struct) 0.3 (`KismetMathLibrary.RandomFloatInRange` 0.65 1.35) 0.0 "/Game/Game_Files/SFX/DistanceSFX.DistanceSFX" null null)
  (bind _asue_4asp_character (cast `/Game/Game_Files/Character/Ue4ASP_Character` (`GameplayStatics.GetPlayerCharacter` 0)))
  (set `/Game/Game_Files/Character/Ue4ASP_Character.BulletInAir?` false _asue_4asp_character)
  (set `/Game/Game_Files/Character/Ue4ASP_Character.Current Mag` (`KismetMathLibrary.Clamp` (+ (`/Game/Game_Files/Character/Ue4ASP_Character.Current Mag` _asue_4asp_character) 1) 0 12) _asue_4asp_character)
  (`self.K2_DestroyActor`))

(event `self.ReceiveHit`
  (params (MyComp :type "PrimitiveComponent Object Reference") (Other :type "Actor Object Reference") (OtherComp :type "PrimitiveComponent Object Reference") (bSelfMoved :type Boolean) (HitLocation :type "Vector Structure") (HitNormal :type "Vector Structure") (NormalImpulse :type "Vector Structure") (Hit :type "HitResult Structure (by ref)"))
  (bind (_returnvalue_roll _returnvalue_pitch _returnvalue_yaw) (`KismetMathLibrary.BreakRotator` (`KismetMathLibrary.Conv_VectorToRotator` HitNormal)))
  (bind _returnvalue (`self.ActorHasTag` Other "T_Spawn"))
  ;[1 1 1] Check Object Hit
  (if (`self.ActorHasTag` Other "Objective")
    (`self.Hit Objective`)
    (else
      (`KismetSystemLibrary.PrintString` (`KismetStringLibrary.Conv_BoolToString` _returnvalue))
      (if _returnvalue
        (if (`self.ActorHasTag` Other "Tramp")
          (`self.Hit Tramp`)
          (else
            (`self.Spawn Tramp` "/Game/Game_Files/Gun/TrampBP.TrampBP_C" (`KismetMathLibrary.MakeRotator` _returnvalue_roll (- _returnvalue_pitch (`self.Angle Change`)) _returnvalue_yaw) (3.0 3.0 1.3))))
        (else
          (bind _asue_4asp_character (cast `/Game/Game_Files/Character/Ue4ASP_Character` (`GameplayStatics.GetPlayerCharacter` 0)))
          (set `/Game/Game_Files/Character/Ue4ASP_Character.BulletInAir?` false _asue_4asp_character)
          (`self.K2_DestroyActor`))))))

(event `self.ReceiveBeginPlay`
  ;[1 1 1] Start
  (`|ExecutionSequence`
    (:`then_0`
      (bind _asue_4asp_character (cast `/Game/Game_Files/Character/Ue4ASP_Character` (`GameplayStatics.GetPlayerCharacter` 0)))
      (bind _output_get (set `/Game/Game_Files/Character/Ue4ASP_Character.BulletRef` self _asue_4asp_character))
      (`KismetSystemLibrary.PrintString` (`KismetSystemLibrary.GetDisplayName` _output_get)))
    (:`then_1`
      (`KismetSystemLibrary.Delay` 1.0)
      (if (`/Game/Game_Files/Character/Ue4ASP_Character.BulletInAir?` _asue_4asp_character)
        (set `/Game/Game_Files/Character/Ue4ASP_Character.BulletInAir?` false _asue_4asp_character)
        (`self.K2_DestroyActor`)))))

(event `Spawn Tramp`
  (params (Tramp :type "Actor Class Reference") (`Spawn Transform Rotation` :type "Rotator Structure") (`Spawn Transform Scale` :type "Vector Structure"))
  ;[1 1 1] Spawn Trampoline
  (`/Engine/EditorBlueprintResources/StandardMacros.DoOnce` false
    (:`Completed`
      (`|SpawnActorFromClass` Tramp (`KismetMathLibrary.MakeTransform` (+ (`SceneComponent.K2_GetComponentLocation` (`self.Sphere`)) (0.0 2.0 0.0)) (`KismetMathLibrary.MakeRotator` `Spawn Transform Rotation_Roll` `Spawn Transform Rotation_Pitch` `Spawn Transform Rotation_Yaw`) `Spawn Transform Scale`) "Undefined" "OverrideRootScale" null null)
      (bind _asue_4asp_character (cast `/Game/Game_Files/Character/Ue4ASP_Character` (`GameplayStatics.GetPlayerCharacter` 0)))
      (`/Game/Game_Files/Character/Ue4ASP_Character.Reset Ball` _asue_4asp_character)
      (`self.K2_DestroyActor`))))

(fn `UserConstructionScript`)